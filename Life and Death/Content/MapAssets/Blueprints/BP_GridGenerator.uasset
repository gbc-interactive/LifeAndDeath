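; BP_GridGenerator builds the hex tile map and picks the tile where the invasive species starts.
; Generate Grids Of Below Size destroys existing BP_HexGrid actors, then spawns GridY by GridX new ones, offsetting alternate rows to form the hex layout.
; A random cell in roughly the upper half of the GridY index range gets flagged as the invasive species spawn, which the tile itself handles on start.
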(fn ConstructionScript)

(fn GenerateGridsOfBelowSize
  (CallFunction|DestroyOldActors)
  (CallFunction|PickRandomISLocation (LocalVariables|GetIS%20Spawn%20Location))
  ;[0 0.1895 1] Grid Map Generator
  (for _index (range 0 (- (Variables|Default|GetGrid%20Y) 1))
    (for _index_2 (range 0 (- (Variables|Default|GetGrid%20X) 1))
      (bind _returnvalue (Game|SpawnActorfromClass "/Game/MapAssets/Blueprints/BP_HexGrid.BP_HexGrid_C" (Math|Transform|MakeTransform (Math|Vector|SelectVector (Math|Vector|MakeVector (* _index (Variables|Default|GetSpacing%20Y)) (* _index_2 (Variables|Default|GetSpacing%20X)) 0.0) (Math|Vector|MakeVector (* _index (Variables|Default|GetSpacing%20Y)) (+ (Variables|Default|GetOffset) (* _index_2 (Variables|Default|GetSpacing%20X))) 0.0) (== (Math|Integer|%(Integer) _index 2) 0)) "0, 0, 0" "1.000000,1.000000,1.000000") "Undefined" "MultiplyWithRoot" 0 0))
      ;[1 1 1] Checks if IS Spawn location and the current tile location are the same, if they are it sets the tile to be IS flag, which is then handled in the BP_Tile script on start. - Ernie Burrows
      (bind _output_get (LocalVariables|SetCurrent%20Tile%20Location (Math|Vector|MakeVector (Math|Conversions|ToFloat(Integer) _index) (Math|Conversions|ToFloat(Integer) _index_2) 0.0)))
      (Variables|/Game/MapAssets/Blueprints/BP_HexGrid.BP_HexGrid_C|SetIs%20Invasice%20Species _returnvalue (Utilities|Operators|EqualEqual (LocalVariables|GetIS%20Spawn%20Location) _output_get 0.0)))))

(fn DestroyOldActors
  ;[1 1 1] Deletes old Actors when new ones are spawned - Ernie Burrows
  (bind _outactors (Actor|GetAllActorsOfClass "/Game/MapAssets/Blueprints/BP_HexGrid.BP_HexGrid_C"))
  (for _array_element _outactors
    (Utilities|IsValid _array_element
      (:Is%20Valid
        (Actor|DestroyActor _array_element)))))

(fn PickRandomISLocation
  (params (NewParam :type Vector%20%28by%20ref%29))
  (bind _grid_y (Variables|Default|GetGrid%20Y))
  ;[1 1 1] Divides grid by 2 along the X (In value so it is truncated) then picks a vector with these bounds, then sets IS location (Vector) to this value - Ernie Burrows
  (Class|KismetMathLibrary|VectorSet NewParam (- (Math|Conversions|ToFloat(Integer) (Math|Random|RandomIntegerinRange (/ _grid_y 2) _grid_y)) 1.0) (- (Math|Conversions|ToFloat(Integer) (Math|Random|RandomIntegerinRange 1 (Variables|Default|GetGrid%20X))) 1.0) 0.0))