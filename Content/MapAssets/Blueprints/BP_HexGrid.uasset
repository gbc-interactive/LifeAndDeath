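; Hex grid tile for a Life-versus-Death game, holding the tile's type and the ecosystem actor on it.
; ChangeTileTypeMaster caches the player's pawn and dispatches to per-type functions.
; Life spends energy to spawn Ocean, Forest or Mountain; emptying follows role-based rules, with errors shown in a temporary widget.
; IS spawns an AI actor, corrupted types only set state, and TileType's OnRep notifies listeners and updates BP_GridGenerator's timer.
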(event Custom|ePrint%20Message%20to%20UI
  (params (Pass%20Message :type String) (Second%20Message :type String))
  ;[1 0 0.5839] Print Message to UI
  (Utilities|FlowControl|Sequence
    (:then_0
      (Utilities|IsValid (Variables|Default|GetMessage%20Widget%20%20Ref)
        (:Is%20Valid
          (Widget|RemovefromParent (Variables|Default|GetMessage%20Widget%20%20Ref)))))
    (:then_1
      (bind _returnvalue (UserInterface|CreateWidget "/Game/MapAssets/UI/WBP_Message.WBP_Message_C"))
      (bind _output_get (Variables|Default|SetMessage%20Widget%20%20Ref _returnvalue))
      (Variables|/Game/MapAssets/UI/WBP_Message.WBP_Message_C|SetMessage _output_get (Utilities|String|Append Pass%20Message Second%20Message))
      (UserInterface|Viewport|AddtoViewport _returnvalue 0)
      (Utilities|FlowControl|Delay 2.0)
      (Widget|RemovefromParent _returnvalue))))

(event EventBeginPlay
  (bind _tile_type (Variables|Default|GetTile%20Type))
  ;[1 1 1] Set tile types of start - Mostly for the IS - Dont Set empty tile, this is already default. Save processing yeah :)
  (Utilities|FlowControl|Delay 0.2)
  (if (!= _tile_type 0)
    (CallFunction|ChangeTileTypeMaster _tile_type)))

(fn ConstructionScript)

(fn ChangeTileTypeMaster
  (params (TileTypeEnum :type Integer))
  (bind _returnvalue (Game|Player|GetPlayerPawn 0))
  ;[1 1 1] Switch statment that runs when ChangeTileTypeMaster is called - Put all logic in specific tile type functions
  (bind _asbp_life (Utilities|Casting|CastToBP_Life _returnvalue)
    (:then
      (Variables|Default|SetCharacterLifeRef _asbp_life)
      (switch int TileTypeEnum :!label _label
        (:0
          (CallFunction|ChangeTiletoEmpty))
        (:1
          (CallFunction|ChangeTiletoForest))
        (:2
          (CallFunction|ChangeTiletoOcean))
        (:3
          (CallFunction|ChangeTiletoMountain))
        (:4
          (CallFunction|ChangeTiletoGraveyard))
        (:5
          (CallFunction|ChangeTiletoIS))
        (:6
          (CallFunction|ChangeTiletoSeedling))
        (:7
          (CallFunction|ChangeTiletoCorruptedOcean))
        (:8
          (CallFunction|ChangeTiletoCorruptedMountain))
        (:9
          (CallFunction|ChangeTiletoCorruptedForest))
        (:10
          (CallFunction|ChangeTiletoCorruptedEmptyTile))))
    (:CastFailed
      (Development|PrintString "Not Playing As Life")
      (bind _asbp_death (Utilities|Casting|CastToBP_Death _returnvalue)
        (:then
          (Variables|Default|SetCharacterDeathRef _asbp_death)
          (goto _label))
        (:CastFailed
          (Development|PrintString "Character Ref Error in BP_HexGrid"))))))

(fn ChangeTiletoIS
  (Variables|/Script/Engine.SkeletalMesh|SetSkeleton (Variables|Default|GetNewVar) "/Game/TaskCharacter/ISCharacters/AdultIS_Optimized_Skeleton.AdultIS_Optimized_Skeleton")
  (bind _returnvalue (Game|SpawnActorfromClass "/Game/TaskCharacter/ThirdPerson/Blueprints/BP_IS2.BP_IS2_C" (Math|Conversions|ToTransform(Vector) (+ (Transformation|GetActorLocation) "0.000000,0.000000,200.000000")) "Undefined" "MultiplyWithRoot" 0 0))
  (Default|SpawnAIController _returnvalue self)
  (Variables|Default|SetTile%20Type 5))

(fn ChangeTiletoEmpty
  (bind _ecosystemactor (Variables|Default|GetEcoSystemActor))
  (if (Utilities|IsValid (Variables|Default|GetCharacterDeathRef))
    (if (Math|Boolean|ORBoolean (== (Variables|Default|GetTile%20Type) 5) (== (Variables|Default|GetTile%20Type) 6) (== (Variables|Default|GetTile%20Type) 7) (== (Variables|Default|GetTile%20Type) 8) (== (Variables|Default|GetTile%20Type) 9))
      (if true :!label _label
        (if (Utilities|IsValid _ecosystemactor)
          (Actor|DestroyActor _ecosystemactor)
          (Variables|Default|SetTile%20Type 0)
          (else
            (Development|PrintString "There is no ecosystem here to destroy")))
        (else
          (Development|PrintString "Not enough energy")))
      (else
        (CallFunction|EPrintMessagetoUI "You can only destroy IS, or corrupted ecosystems as death")))
    (elif (Math|Boolean|ORBoolean (== (Variables|Default|GetTile%20Type) 1) (== (Variables|Default|GetTile%20Type) 2) (== (Variables|Default|GetTile%20Type) 3))
      (goto _label)
      (else
        (CallFunction|EPrintMessagetoUI "You can only destroy Ocean, Mountain or Forest")))))

(fn ChangeTiletoOcean
  (bind _characterliferef (Variables|Default|GetCharacterLifeRef))
  (bind _characterliferef_2 (Variables|Default|GetCharacterLifeRef))
  (Utilities|IsValid (Variables|Default|GetCharacterLifeRef)
    (:Is%20Valid
      (if (== (Variables|Default|GetTile%20Type) 0)
        (if (> (Variables|/Game/TaskCharacter/ThirdPerson/Blueprints/BP_Life.BP_Life_C|GetCurrent%20Energy _characterliferef) (Variables|/Game/TaskCharacter/ThirdPerson/Blueprints/BP_Life.BP_Life_C|GetSpawnOceanEcosystemCost _characterliferef))
          (bind _returnvalue (Game|SpawnActorfromClass "/Game/MapAssets/Blueprints/BP_Object_2.BP_Object_2_C" (Transformation|GetWorldTransform (Variables|Default|GetStaticMesh)) "Undefined" "OverrideRootScale" 0 0))
          (Variables|Default|SetEcoSystemActor _returnvalue)
          (Variables|Default|SetTile%20Type 2)
          ;[0.04627 1 0] Updating Life's Energy System
          (Default|ELockoutTimer _characterliferef_2 3.0)
          (Default|DeductEnergyCost _characterliferef_2 "NewEnumerator1")
          (Variables|/Game/TaskCharacter/ThirdPerson/Blueprints/BP_Life.BP_Life_C|SetNoOfOceanEcosystems _characterliferef_2 (+ (Variables|/Game/TaskCharacter/ThirdPerson/Blueprints/BP_Life.BP_Life_C|GetNoOfOceanEcosystems _characterliferef_2) 1.0))
          (else
            (CallFunction|EPrintMessagetoUI "Insufficient Energy, Required Energy " (Utilities|String|ToString(Float) (Variables|/Game/TaskCharacter/ThirdPerson/Blueprints/BP_Life.BP_Life_C|GetSpawnOceanEcosystemCost (Variables|Default|GetCharacterLifeRef))))))
        (else
          (CallFunction|EPrintMessagetoUI "Cannot create tile here it's current tile type is:" (Utilities|String|ToString(Integer) (Variables|Default|GetTile%20Type))))))))

(fn ChangeTiletoForest
  (bind _characterliferef (Variables|Default|GetCharacterLifeRef))
  (bind _characterliferef_2 (Variables|Default|GetCharacterLifeRef))
  (Utilities|IsValid (Variables|Default|GetCharacterLifeRef)
    (:Is%20Valid
      (if (== (Variables|Default|GetTile%20Type) 0)
        (if (> (Variables|/Game/TaskCharacter/ThirdPerson/Blueprints/BP_Life.BP_Life_C|GetCurrent%20Energy _characterliferef) (Variables|/Game/TaskCharacter/ThirdPerson/Blueprints/BP_Life.BP_Life_C|GetSpawnForestEcosystemCost _characterliferef))
          (bind _returnvalue (Game|SpawnActorfromClass "/Game/MapAssets/Blueprints/BP_Object_1.BP_Object_1_C" (Transformation|GetWorldTransform (Variables|Default|GetStaticMesh)) "Undefined" "OverrideRootScale" 0 0))
          (Variables|Default|SetEcoSystemActor _returnvalue)
          (Variables|Default|SetTile%20Type 1)
          ;[0.04627 1 0] Updating Life's Energy System
          (Default|ELockoutTimer _characterliferef_2 5.0)
          (Default|DeductEnergyCost _characterliferef_2 "NewEnumerator0")
          (Variables|/Game/TaskCharacter/ThirdPerson/Blueprints/BP_Life.BP_Life_C|SetNoOfForestEcosystems _characterliferef_2 (+ (Variables|/Game/TaskCharacter/ThirdPerson/Blueprints/BP_Life.BP_Life_C|GetNoOfForestEcosystems _characterliferef_2) 1.0))
          (else
            (CallFunction|EPrintMessagetoUI "Insufficient Energy, Required Energy " (Utilities|String|ToString(Float) (Variables|/Game/TaskCharacter/ThirdPerson/Blueprints/BP_Life.BP_Life_C|GetSpawnForestEcosystemCost (Variables|Default|GetCharacterLifeRef))))))
        (else
          (CallFunction|EPrintMessagetoUI "Cannot create tile here it's current tile type is:" (Utilities|String|ToString(Integer) (Variables|Default|GetTile%20Type))))))))

(fn ChangeTiletoMountain
  (bind _characterliferef (Variables|Default|GetCharacterLifeRef))
  (bind _characterliferef_2 (Variables|Default|GetCharacterLifeRef))
  (Utilities|IsValid (Variables|Default|GetCharacterLifeRef)
    (:Is%20Valid
      (if (== (Variables|Default|GetTile%20Type) 0)
        (if (> (Variables|/Game/TaskCharacter/ThirdPerson/Blueprints/BP_Life.BP_Life_C|GetCurrent%20Energy _characterliferef) (Variables|/Game/TaskCharacter/ThirdPerson/Blueprints/BP_Life.BP_Life_C|GetSpawnMountainEcosystemCost _characterliferef))
          (bind _returnvalue (Game|SpawnActorfromClass "/Game/MapAssets/Blueprints/BP_Object_3.BP_Object_3_C" (Transformation|GetWorldTransform (Variables|Default|GetStaticMesh)) "Undefined" "OverrideRootScale" 0 0))
          (Variables|Default|SetEcoSystemActor _returnvalue)
          (Variables|Default|SetTile%20Type 3)
          ;[0.04627 1 0] Updating Life's Energy System
          (Default|ELockoutTimer _characterliferef_2 7.0)
          (Default|DeductEnergyCost _characterliferef_2 "NewEnumerator2")
          (Variables|/Game/TaskCharacter/ThirdPerson/Blueprints/BP_Life.BP_Life_C|SetNoOfMountainEcosystems _characterliferef_2 (+ (Variables|/Game/TaskCharacter/ThirdPerson/Blueprints/BP_Life.BP_Life_C|GetNoOfMountainEcosystems _characterliferef_2) 1.0))
          (else
            (CallFunction|EPrintMessagetoUI "Insufficient Energy, Required Energy " (Utilities|String|ToString(Float) (Variables|/Game/TaskCharacter/ThirdPerson/Blueprints/BP_Life.BP_Life_C|GetSpawnMountainEcosystemCost (Variables|Default|GetCharacterLifeRef))))))
        (else
          (CallFunction|EPrintMessagetoUI "Cannot create tile here it's current tile type is:" (Utilities|String|ToString(Integer) (Variables|Default|GetTile%20Type))))))))

(fn ChangeTiletoGraveyard
  (bind _characterdeathref (Variables|Default|GetCharacterDeathRef))
  (Utilities|IsValid _characterdeathref
    (:Is%20Valid
      (if (> (Variables|/Game/TaskCharacter/ThirdPerson/Blueprints/BP_Death.BP_Death_C|GetCurrent%20Energy _characterdeathref) 0.0)
        (Variables|Default|SetTile%20Type 4)))
    (:Is%20Not%20Valid
      (Development|PrintString "Invalid Character Reference in BP_HexGrid"))))

(fn ChangeTiletoSeedling
  (Variables|Default|SetTile%20Type 6)
  (Variables|Default|SetEcoSystemActor 0))

(fn ChangeTiletoCorruptedOcean
  (Variables|Default|SetTile%20Type 7))

(fn ChangeTiletoCorruptedForest
  (Variables|Default|SetTile%20Type 9))

(fn ChangeTiletoCorruptedMountain
  (Variables|Default|SetTile%20Type 8))

(fn ChangeTiletoCorruptedEmptyTile
  (Variables|Default|SetTile%20Type 10))

(fn OnRepTileType
  (Utilities|FlowControl|Sequence
    (:then_0
      (if (Math|Integer|InRange(Integer) (Variables|Default|GetTile%20Type) 1 3)
        (Default|CallOnTypeChange self)))
    (:then_1
      (if (Math|Integer|InRange(Integer) (Variables|Default|GetTile%20Type) 5 6)
        (bind _returnvalue (Actor|GetActorOfClass "/Game/MapAssets/Blueprints/BP_GridGenerator.BP_GridGenerator_C"))
        (Default|ToogleTimer _returnvalue false)
        (else
          (bind _outactors (Actor|GetAllActorsOfClass "BP_HexGrid_C"))
          (bind _array_element (Utilities|Array|ForEachLoopwithBreak _outactors :!label _label)
            (:LoopBody
              (if (Math|Integer|InRange(Integer) (Variables|BP_HexGrid_C|GetTile%20Type _array_element) 5 6)
                (bind _returnvalue_2 (Actor|GetActorOfClass "/Game/MapAssets/Blueprints/BP_GridGenerator.BP_GridGenerator_C"))
                (Variables|/Game/MapAssets/Blueprints/BP_GridGenerator.BP_GridGenerator_C|SetisTileSpecial _returnvalue_2 true)
                (Default|CheckAllBooleans _returnvalue_2)
                (goto _label Break)))
            (:Completed
              (Variables|/Game/MapAssets/Blueprints/BP_GridGenerator.BP_GridGenerator_C|SetisTileSpecial _returnvalue_2 false)
              (Default|ToogleTimer _returnvalue_2 false))))))))

(fn Checkif)