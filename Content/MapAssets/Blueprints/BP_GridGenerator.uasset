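; Grid generator Blueprint that builds the hex tile map at BeginPlay and seeds one invasive species tile.
; It destroys existing BP_HexGrid actors, fills TileSpawnLocations with row positions staggered by Offset, then spawns a tile at each.
; A random index from the second half of the array marks the invasive tile, though the inclusive maximum can fall past the last tile.
; CreateAIMap is called afterwards but is an empty stub.
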(event EventBeginPlay
  (CallFunction|GenerateGridsOfBelowSize)
  (CallFunction|CreateAIMap "0, 0, 0"))

(fn ConstructionScript)

(fn GenerateGridsOfBelowSize
  (CallFunction|DestroyOldActors)
  ;[1 1 1] Set the Array size based on grid X and Y size
  (Utilities|Array|Resize (Variables|Default|GetTile%20Spawn%20Locations) (* (Variables|Default|GetGrid%20Y) (Variables|Default|GetGrid%20X)))
  ;[0 0.1895 1] Grid Map Generator
  (for _index (range 0 (- (Variables|Default|GetGrid%20Y) 1))
    (for _index_2 (range 0 (- (Variables|Default|GetGrid%20X) 1))
      (bind _result (Math|Integer|IncrementInt (Variables|Default|Getint))
        (:%20%20
          (Utilities|Array|SetArrayElem (Variables|Default|GetTile%20Spawn%20Locations) _result (Math|Vector|SelectVector (Math|Vector|MakeVector (* _index (Variables|Default|GetSpacing%20Y)) (* _index_2 (Variables|Default|GetSpacing%20X)) 0.0) (Math|Vector|MakeVector (* _index (Variables|Default|GetSpacing%20Y)) (+ (Variables|Default|GetOffset) (* _index_2 (Variables|Default|GetSpacing%20X))) 0.0) (== (Math|Integer|%(Integer) _index 2) 0)))))))
  (bind _indexforis (CallFunction|PickRandomISLocation))
  ;[1 1 1] Spawn the tiles at TileSpawnLocations array and set the invasive species tile's enum
  (for (_array_element _array_index) (Variables|Default|GetTile%20Spawn%20Locations)
    (bind _returnvalue (Game|SpawnActorfromClass "/Game/MapAssets/Blueprints/BP_HexGrid.BP_HexGrid_C" (Math|Transform|MakeTransform _array_element "0, 0, 0" "1.000000,1.000000,1.000000") "Undefined" "MultiplyWithRoot" 0 0))
    (if (== _indexforis _array_index)
      (Variables|/Game/MapAssets/Blueprints/BP_HexGrid.BP_HexGrid_C|SetTile%20Type _returnvalue 5))))

(fn DestroyOldActors
  ;[1 1 1] Deletes old Actors when new ones are spawned - Ernie Burrows
  (bind _outactors (Actor|GetAllActorsOfClass "/Game/MapAssets/Blueprints/BP_HexGrid.BP_HexGrid_C"))
  (for _array_element _outactors
    (Utilities|IsValid _array_element
      (:Is%20Valid
        (Actor|DestroyActor _array_element)))))

(fn PickRandomISLocation
  (bind _grid_x (Variables|Default|GetGrid%20X))
  (bind _grid_y (Variables|Default|GetGrid%20Y))
  (bind _returnvalue (* _grid_x _grid_y))
  ;[1 1 1] Divides grid by 2 along the X (In value so it is truncated) then picks a vector with these bounds, then sets IS location (Vector) to this value - Ernie Burrows
  (return (Math|Random|RandomIntegerinRange (/ _returnvalue 2) _returnvalue)))

(fn SetElement2D)

(fn ArrayIndexfromDimensions
  (params (X%20Location :type Integer) (Y%20Location :type Integer))
  (bind _grid_x (Variables|Default|GetGrid%20X))
  (bind _returnvalue (* X%20Location _grid_x))
  (bind _returnvalue_2 (+ _returnvalue Y%20Location))
  (if (< _returnvalue_2 (Utilities|Array|Length (Variables|Default|GetTile%20Spawn%20Locations)))
    (return _returnvalue_2)
    (else
      (Development|PrintString "Index out of bounds"))))

(fn CreateAIMap
  (params (Center :type Vector)))