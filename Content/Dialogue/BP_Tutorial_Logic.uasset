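; Sequences the two-player Life and Death tutorial, showing WBP_Tutorial pages and later the WBP_Energy widget.
; A TaskCounter state machine advances on the controller A button, while Tick moves it on when spawn or ability tasks complete.
; Steps toggle input flags, spawn or move tutorial actors, highlight ability tiles and blend both players to cinematic cameras.
; Seedling growth is an instant scale change, as the Timeline version is never run.
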(event Custom|Switch%20Camera%20focusing%20Seedling
  (bind _returnvalue (Game|GetPlayerController 0))
  ;[1 1 1] Seeding
  (bind _returnvalue_2 (Actor|GetActorOfClass "/Game/Dialogue/Assets/IS/BP_Seedling_Camera.BP_Seedling_Camera_C"))
  (Game|Player|SetViewTargetwithBlend _returnvalue _returnvalue_2 2.0 "VTBlend_PreBlended" 0.0 true)
  (Class|PlayerController|SetCinematicMode _returnvalue true false true true true)
  (bind _returnvalue_3 (Game|SpawnActorfromClass "/Game/Dialogue/BP_Tutorial_Seeding.BP_Tutorial_Seeding_C" (Math|Transform|MakeTransform "90712.230268,1020.000002,-22240.000000" "0, 0, 0" "0.300000,0.300000,0.300000") "Undefined" "MultiplyWithRoot" 0 0)))

(event Custom|Start%20Seedling%20Maturing
  ;[1 1 1] Seeding
  (Transformation|SetActorScale3D (stale Custom|Switch%20Camera%20focusing%20Seedling _returnvalue_3) "1.500000,1.500000,1.500000"))

(event Custom|Exit%20from%20Seedling%20maturing%20camera
  (bind _returnvalue (Game|GetPlayerController 0))
  ;[1 1 1] Seeding
  (Game|Player|SetViewTargetwithBlend _returnvalue (Game|GetPlayerCharacter 0) 2.0 "VTBlend_PreBlended" 0.0 true)
  (Class|PlayerController|SetCinematicMode _returnvalue false false true true true))

(event Custom|Switch%20Camera%20focusing%20IS%20Death
  (bind _returnvalue (Game|GetPlayerController 1))
  ;[1 1 1] IS SPawning Death
  (bind _returnvalue_2 (Actor|GetActorOfClass "/Game/Dialogue/Assets/IS/BP_IS_Camera.BP_IS_Camera_C"))
  (Game|Player|SetViewTargetwithBlend _returnvalue _returnvalue_2 2.0 "VTBlend_PreBlended" 0.0 true)
  (Class|PlayerController|SetCinematicMode _returnvalue true false true true true))

(event Custom|Exit%20from%20IS%20camera%20Death
  (bind _returnvalue (Game|GetPlayerController 1))
  ;[1 1 1] IS SPawning Death
  (Game|Player|SetViewTargetwithBlend _returnvalue (Game|GetPlayerCharacter 1) 2.0 "VTBlend_PreBlended" 0.0 true)
  (Class|PlayerController|SetCinematicMode _returnvalue false false true true true)
  (Variables|Default|SetBackToMainCamera? true))

(event Custom|Switch%20Camera%20focusing%20Seedling%20Death
  (bind _returnvalue (Game|GetPlayerController 1))
  ;[1 1 1] Seeding Death
  (bind _returnvalue_2 (Actor|GetActorOfClass "/Game/Dialogue/Assets/IS/BP_Seedling_Camera.BP_Seedling_Camera_C"))
  (Game|Player|SetViewTargetwithBlend _returnvalue _returnvalue_2 2.0 "VTBlend_PreBlended" 0.0 true)
  (Class|PlayerController|SetCinematicMode _returnvalue true false true true true))

(event Custom|Exit%20from%20Seedling%20maturing%20camera%20Death
  (bind _returnvalue (Game|GetPlayerController 1))
  ;[1 1 1] Seeding Death
  (Game|Player|SetViewTargetwithBlend _returnvalue (Game|GetPlayerCharacter 1) 2.0 "VTBlend_PreBlended" 0.0 true)
  (Class|PlayerController|SetCinematicMode _returnvalue false false true true true))

(event Custom|Switch%20Camera%20focusing%20IS
  (bind _returnvalue (Game|GetPlayerController 0))
  ;[1 1 1] IS SPawning
  (bind _returnvalue_2 (Actor|GetActorOfClass "/Game/Dialogue/Assets/IS/BP_IS_Camera.BP_IS_Camera_C"))
  (Game|Player|SetViewTargetwithBlend _returnvalue _returnvalue_2 2.0 "VTBlend_PreBlended" 0.0 true)
  (Class|PlayerController|SetCinematicMode _returnvalue true false true true true)
  (Game|SpawnActorfromClass "/Game/Dialogue/BP_Tutorial_IS.BP_Tutorial_IS_C" (Math|Transform|MakeTransform "90728.383086,3920.000001,-22280.000000" "0, 0, 0" "1.000000,1.000000,1.000000") "Undefined" "MultiplyWithRoot" 0 0))

(event Custom|Exit%20from%20IS%20camera
  (bind _returnvalue (Game|GetPlayerController 0))
  ;[1 1 1] IS SPawning
  (Game|Player|SetViewTargetwithBlend _returnvalue (Game|GetPlayerCharacter 0) 2.0 "VTBlend_PreBlended" 0.0 true)
  (Class|PlayerController|SetCinematicMode _returnvalue false false true true true)
  (Variables|Default|SetBackToMainCamera? true))

(event Input|EnhancedActionEvents|EnhancedInputActionTutorial_Controller_A
  (params (ActionValue :type Boolean) (ElapsedSeconds :type Float%20%28double-precision%29) (TriggeredSeconds :type Float%20%28double-precision%29) (InputAction :type Input%20Action%20Object%20Reference :default "/Game/Dialogue/Assets/Input/IMC/Tutorial_Controller_A.Tutorial_Controller_A"))
  (bind _wbp_tutorial_ref (Variables|Default|GetWBP_Tutorial%20Ref))
  (bind _wbp_tutorial_ref_2 (Variables|Default|GetWBP_Tutorial%20Ref))
  (bind _wbp_tutorial_ref_3 (Variables|Default|GetWBP_Tutorial%20Ref))
  (bind _wbp_tutorial_ref_4 (Variables|Default|GetWBP_Tutorial%20Ref))
  (bind _wbp_tutorial_ref_5 (Variables|Default|GetWBP_Tutorial%20Ref))
  (bind _wbp_tutorial_ref_6 (Variables|Default|GetWBP_Tutorial%20Ref))
  (bind _wbp_tutorial_ref_7 (Variables|Default|GetWBP_Tutorial%20Ref))
  (bind _wbp_tutorial_ref_8 (Variables|Default|GetWBP_Tutorial%20Ref))
  (bind _wbp_tutorial_ref_9 (Variables|Default|GetWBP_Tutorial%20Ref))
  (bind _wbp_tutorial_ref_10 (Variables|Default|GetWBP_Tutorial%20Ref))
  (bind _wbp_tutorial_ref_11 (Variables|Default|GetWBP_Tutorial%20Ref))
  (bind _wbp_tutorial_ref_12 (Variables|Default|GetWBP_Tutorial%20Ref))
  (bind _wbp_tutorial_ref_13 (Variables|Default|GetWBP_Tutorial%20Ref))
  (bind _wbp_tutorial_ref_14 (Variables|Default|GetWBP_Tutorial%20Ref))
  (bind _wbp_tutorial_ref_15 (Variables|Default|GetWBP_Tutorial%20Ref))
  (bind _wbp_tutorial_ref_16 (Variables|Default|GetWBP_Tutorial%20Ref))
  (bind _wbp_tutorial_ref_17 (Variables|Default|GetWBP_Tutorial%20Ref))
  (bind _wbp_tutorial_ref_18 (Variables|Default|GetWBP_Tutorial%20Ref))
  (bind _canvas2 (Variables|/Game/Dialogue/WBP_Tutorial.WBP_Tutorial_C|GetCanvas2 _wbp_tutorial_ref_3))
  (bind _7 (Variables|/Game/Dialogue/WBP_Tutorial.WBP_Tutorial_C|Get7 _wbp_tutorial_ref_10))
  (bind _8 (Variables|/Game/Dialogue/WBP_Tutorial.WBP_Tutorial_C|Get8 _wbp_tutorial_ref_14))
  (switch int (Variables|Default|GetTask_Counter)
    (:0
      (Widget|SetVisibility (Variables|/Game/Dialogue/WBP_Tutorial.WBP_Tutorial_C|GetCanvas1 _wbp_tutorial_ref) "Hidden")
      (Widget|SetVisibility (Variables|/Game/Dialogue/WBP_Tutorial.WBP_Tutorial_C|GetCanvas2 _wbp_tutorial_ref) "Visible")
      (Variables|Default|SetTask_Counter 1))
    (:1
      (Utilities|FlowControl|FlipFlop
        (:A
          (Widget|SetVisibility _canvas2 "Hidden"))
        (:B
          (Widget|SetVisibility _canvas2 "Visible"))))
    (:2
      (Widget|SetVisibility (Variables|/Game/Dialogue/WBP_Tutorial.WBP_Tutorial_C|Get6 _wbp_tutorial_ref_13) "Hidden")
      (Widget|SetVisibility (Variables|/Game/Dialogue/WBP_Tutorial.WBP_Tutorial_C|Get6D _wbp_tutorial_ref_13) "Hidden")
      (Widget|SetVisibility (Variables|/Game/Dialogue/WBP_Tutorial.WBP_Tutorial_C|Get7 _wbp_tutorial_ref_13) "Visible")
      (Variables|Default|SetENable%20Input%20Life true)
      (Variables|Default|SetTask_Counter 3))
    (:3
      (Utilities|FlowControl|FlipFlop
        (:A
          (Widget|SetVisibility _7 "Hidden"))
        (:B
          (Widget|SetVisibility _7 "Visible"))))
    (:4
      (Utilities|FlowControl|FlipFlop
        (:A
          (Widget|SetVisibility _8 "Hidden"))
        (:B
          (Widget|SetVisibility _8 "Visible"))))
    (:5
      (Utilities|FlowControl|DoOnce false
        (:Completed
          (Widget|SetVisibility (Variables|/Game/Dialogue/WBP_Tutorial.WBP_Tutorial_C|Get9 _wbp_tutorial_ref_11) "Hidden")
          (Widget|SetVisibility (Variables|/Game/Dialogue/WBP_Tutorial.WBP_Tutorial_C|Get9D _wbp_tutorial_ref_11) "Hidden")
          (bind _returnvalue (UserInterface|CreateWidget "/Game/Dialogue/WBP_Energy.WBP_Energy_C"))
          (bind _output_get (Variables|Default|SetWBP_Energy%20Ref _returnvalue))
          (UserInterface|Viewport|AddtoViewport _output_get 0)
          (Utilities|FlowControl|Delay 3.0)
          (Widget|SetVisibility (Variables|/Game/Dialogue/WBP_Energy.WBP_Energy_C|Get1 (Variables|Default|GetWBP_Energy%20Ref)) "Hidden")
          (Widget|SetVisibility (Variables|/Game/Dialogue/WBP_Tutorial.WBP_Tutorial_C|Get10 (Variables|Default|GetWBP_Tutorial%20Ref)) "Visible")
          (Variables|Default|SetTask_Counter 6))))
    (:6
      (Utilities|FlowControl|DoOnce false
        (:Completed
          (Widget|SetVisibility (Variables|/Game/Dialogue/WBP_Tutorial.WBP_Tutorial_C|Get10 (Variables|Default|GetWBP_Tutorial%20Ref)) "Hidden")
          (CallFunction|SwitchCameraFocusingIS)
          (CallFunction|SwitchCameraFocusingISDeath)
          (Utilities|FlowControl|Delay 3.0)
          (Widget|SetVisibility (Variables|/Game/Dialogue/WBP_Tutorial.WBP_Tutorial_C|Get11 (Variables|Default|GetWBP_Tutorial%20Ref)) "Visible")
          (Variables|Default|SetTask_Counter 7))))
    (:7
      (Widget|SetVisibility (Variables|/Game/Dialogue/WBP_Tutorial.WBP_Tutorial_C|Get11 _wbp_tutorial_ref_9) "Hidden")
      (Widget|SetVisibility (Variables|/Game/Dialogue/WBP_Tutorial.WBP_Tutorial_C|Get12 _wbp_tutorial_ref_9) "Visible")
      (Variables|Default|SetTask_Counter 8))
    (:8
      (CallFunction|ExitfromISCamera)
      (CallFunction|ExitfromISCameraDeath)
      (bind _returnvalue_2 (Game|SpawnActorfromClass "/Game/MapAssets/Blueprints/BP_Object_1.BP_Object_1_C" (Math|Transform|MakeTransform "1204.804925,701.914712,62.472575" "0.000000,29.500000,0.000000" "1.000000,1.000000,1.000000") "Undefined" "MultiplyWithRoot" 0 0))
      (Widget|SetVisibility (Variables|/Game/Dialogue/WBP_Tutorial.WBP_Tutorial_C|Get12 _wbp_tutorial_ref_15) "Hidden")
      (Widget|SetVisibility (Variables|/Game/Dialogue/WBP_Tutorial.WBP_Tutorial_C|Get13 _wbp_tutorial_ref_15) "Visible")
      (Variables|Default|SetTask_Counter 9))
    (:9
      (Utilities|FlowControl|DoOnce false
        (:Completed
          (Actor|DestroyActor _returnvalue_2)
          (Game|SpawnActorfromClass "/Game/MapAssets/Blueprints/BP_ForestGraveyard.BP_ForestGraveyard_C" (Math|Transform|MakeTransform "1223.283468,681.575127,63.429784" "0.000000,29.500000,0.000000" "1.000000,1.000000,1.000000") "Undefined" "MultiplyWithRoot" 0 0)
          (Widget|SetVisibility (Variables|/Game/Dialogue/WBP_Tutorial.WBP_Tutorial_C|Get13 (Variables|Default|GetWBP_Tutorial%20Ref)) "Hidden")
          (Utilities|FlowControl|Delay 3.0)
          (Widget|SetVisibility (Variables|/Game/Dialogue/WBP_Tutorial.WBP_Tutorial_C|Get14 (Variables|Default|GetWBP_Tutorial%20Ref)) "Visible")
          (Variables|Default|SetTask_Counter 10))))
    (:10
      (Utilities|FlowControl|DoOnce false
        (:Completed
          (Widget|SetVisibility (Variables|/Game/Dialogue/WBP_Tutorial.WBP_Tutorial_C|Get14 (Variables|Default|GetWBP_Tutorial%20Ref)) "Hidden")
          (CallFunction|SwitchCameraFocusingSeedling)
          (CallFunction|SwitchCameraFocusingSeedlingDeath)
          (Utilities|FlowControl|Delay 3.0)
          (Widget|SetVisibility (Variables|/Game/Dialogue/WBP_Tutorial.WBP_Tutorial_C|Get15 (Variables|Default|GetWBP_Tutorial%20Ref)) "Visible")
          (Variables|Default|SetTask_Counter 11))))
    (:11
      (Utilities|FlowControl|DoOnce false
        (:Completed
          (Widget|SetVisibility (Variables|/Game/Dialogue/WBP_Tutorial.WBP_Tutorial_C|Get15 (Variables|Default|GetWBP_Tutorial%20Ref)) "Hidden")
          (CallFunction|StartSeedlingMaturing)
          (Utilities|FlowControl|Delay 3.0)
          (CallFunction|ExitfromSeedlingMaturingCamera)
          (CallFunction|ExitfromSeedlingMaturingCameraDeath)
          (Widget|SetVisibility (Variables|/Game/Dialogue/WBP_Tutorial.WBP_Tutorial_C|Get25 _wbp_tutorial_ref_12) "Visible")
          (Widget|SetVisibility (Variables|/Game/Dialogue/WBP_Energy.WBP_Energy_C|Get1 (Variables|Default|GetWBP_Energy%20Ref)) "Visible")
          (Utilities|FlowControl|Delay 3.0)
          (Widget|SetVisibility (Variables|/Game/Dialogue/WBP_Tutorial.WBP_Tutorial_C|Get25 _wbp_tutorial_ref_12) "Hidden")
          (Widget|SetVisibility (Variables|/Game/Dialogue/WBP_Tutorial.WBP_Tutorial_C|Get16 _wbp_tutorial_ref_16) "Visible")
          (Widget|SetVisibility (Variables|/Game/Dialogue/WBP_Tutorial.WBP_Tutorial_C|Get17 _wbp_tutorial_ref_16) "Visible")
          (Variables|Default|SetTask_Counter 12))))
    (:12
      (Widget|SetVisibility (Variables|/Game/Dialogue/WBP_Tutorial.WBP_Tutorial_C|Get16 _wbp_tutorial_ref_17) "Hidden")
      (Widget|SetVisibility (Variables|/Game/Dialogue/WBP_Tutorial.WBP_Tutorial_C|Get17 _wbp_tutorial_ref_17) "Hidden")
      (bind _returnvalue_3 (Actor|GetActorOfClass "/Game/Dialogue/BP_DeathTutorial.BP_DeathTutorial_C"))
      (Variables|/Game/Dialogue/BP_DeathTutorial.BP_DeathTutorial_C|SetCan%20Use%20ABility1? _returnvalue_3 true)
      (Transformation|SetActorLocation (Variables|Default|GetIS%201%20for%20Ability%201%20ref) "1200.980233,1393.353878,72.124323" false false)
      (Rendering|Material|CreateDynamicMaterialInstance (Variables|/Game/MapAssets/Blueprints/BP_HexGrid.BP_HexGrid_C|GetRed%20Tile (Variables|Default|GetAbility%201%20glow%20tile)) 0 "/Game/MapAssets/Blueprints/Outline_Material.Outline_Material" "None" :!class /Script/Engine.PrimitiveComponent))
    (:13
      (Widget|SetVisibility (Variables|/Game/Dialogue/WBP_Tutorial.WBP_Tutorial_C|Get18 _wbp_tutorial_ref_18) "Hidden")
      (Widget|SetVisibility (Variables|/Game/Dialogue/WBP_Tutorial.WBP_Tutorial_C|Get19 _wbp_tutorial_ref_18) "Hidden")
      (Transformation|SetActorLocation (Variables|Default|GetIS%201%20for%20Ability%202%20ref) "605.753814,1821.908673,92.124361" false false)
      (Transformation|SetActorLocation (Variables|Default|GetIS%202%20for%20Ability%202%20ref_0) "-3.773447,2124.346637,92.124361" false false)
      (Transformation|SetActorLocation (Variables|Default|GetIS%203%20for%20Ability%202%20ref_1) "26.384378,2813.568351,92.124361" false false)
      (Transformation|SetActorLocation (Variables|Default|GetIS%204%20for%20Ability%202%20ref_2) "594.783748,3147.912120,92.124361" false false)
      (Transformation|SetActorLocation (Variables|Default|GetIS%205%20for%20Ability%202%20ref_3) "1179.109525,2888.819508,92.124361" false false)
      (Transformation|SetActorLocation (Variables|Default|GetIS%206%20for%20Ability%202%20ref_4) "1183.045073,2188.065796,92.124361" false false)
      (bind _returnvalue_4 (Actor|GetActorOfClass "/Game/Dialogue/BP_DeathTutorial.BP_DeathTutorial_C"))
      (Variables|/Game/Dialogue/BP_DeathTutorial.BP_DeathTutorial_C|SetCan%20Use%20ABility2? _returnvalue_4 true)
      (Rendering|Material|CreateDynamicMaterialInstance (Variables|/Game/MapAssets/Blueprints/BP_HexGrid.BP_HexGrid_C|GetRed%20Tile (Variables|Default|GetAbility%202%20glow%20tile_0)) 0 "/Game/MapAssets/Blueprints/Outline_Material.Outline_Material" "None" :!class /Script/Engine.PrimitiveComponent))
    (:15
      (Utilities|FlowControl|DoOnce false
        (:Completed
          (Widget|SetVisibility (Variables|/Game/Dialogue/WBP_Tutorial.WBP_Tutorial_C|Get20 _wbp_tutorial_ref_4) "Hidden")
          (Widget|SetVisibility (Variables|/Game/Dialogue/WBP_Tutorial.WBP_Tutorial_C|Get20D _wbp_tutorial_ref_4) "Hidden")
          (Widget|SetVisibility (Variables|/Game/Dialogue/WBP_Energy.WBP_Energy_C|Get2 (Variables|Default|GetWBP_Energy%20Ref)) "Visible")
          (Utilities|FlowControl|Delay 3.0)
          (Widget|SetVisibility (Variables|/Game/Dialogue/WBP_Energy.WBP_Energy_C|Get3 (Variables|Default|GetWBP_Energy%20Ref)) "Visible")
          (Utilities|FlowControl|Delay 3.0)
          (Widget|SetVisibility (Variables|/Game/Dialogue/WBP_Energy.WBP_Energy_C|Get3 (Variables|Default|GetWBP_Energy%20Ref)) "Hidden")
          (Variables|Default|SetTask_Counter 16))))
    (:16
      (Widget|SetVisibility (Variables|/Game/Dialogue/WBP_Tutorial.WBP_Tutorial_C|Get20 _wbp_tutorial_ref_6) "Hidden")
      (Widget|SetVisibility (Variables|/Game/Dialogue/WBP_Tutorial.WBP_Tutorial_C|Get20D _wbp_tutorial_ref_6) "Hidden")
      (Widget|SetVisibility (Variables|/Game/Dialogue/WBP_Tutorial.WBP_Tutorial_C|Get21 _wbp_tutorial_ref_7) "Visible")
      (Widget|SetVisibility (Variables|/Game/Dialogue/WBP_Tutorial.WBP_Tutorial_C|Get21D _wbp_tutorial_ref_7) "Visible")
      (Variables|Default|SetTask_Counter 17))
    (:17
      (Widget|SetVisibility (Variables|/Game/Dialogue/WBP_Tutorial.WBP_Tutorial_C|Get21 _wbp_tutorial_ref_8) "Hidden")
      (Widget|SetVisibility (Variables|/Game/Dialogue/WBP_Tutorial.WBP_Tutorial_C|Get21D _wbp_tutorial_ref_8) "Hidden")
      (Widget|SetVisibility (Variables|/Game/Dialogue/WBP_Tutorial.WBP_Tutorial_C|Get22 _wbp_tutorial_ref_2) "Visible")
      (Widget|SetVisibility (Variables|/Game/Dialogue/WBP_Tutorial.WBP_Tutorial_C|Get22D _wbp_tutorial_ref_2) "Visible")
      (Variables|Default|SetTask_Counter 18))
    (:18
      (Widget|SetVisibility (Variables|/Game/Dialogue/WBP_Tutorial.WBP_Tutorial_C|Get22 _wbp_tutorial_ref_5) "Hidden")
      (Widget|SetVisibility (Variables|/Game/Dialogue/WBP_Tutorial.WBP_Tutorial_C|Get22D _wbp_tutorial_ref_5) "Hidden")
      (Variables|Default|SetTask_Counter 18))))

(event EventBeginPlay
  ;[0.0999 0 1] Comment
  (Utilities|FlowControl|Sequence
    (:then_0
      (bind _returnvalue (Actor|GetActorOfClass "/Game/Dialogue/BP_LifeTutorial.BP_LifeTutorial_C"))
      (Variables|Default|SetBP_Life%20tutorial%20Ref _returnvalue)
      (bind _returnvalue_2 (Actor|GetActorOfClass "/Game/Dialogue/BP_DeathTutorial.BP_DeathTutorial_C"))
      (Variables|Default|SetBP_Death%20Tutorial%20Ref _returnvalue_2))
    (:then_1
      (Utilities|FlowControl|Delay 1.0)
      (bind _returnvalue_3 (UserInterface|CreateWidget "/Game/Dialogue/WBP_Tutorial.WBP_Tutorial_C"))
      (bind _output_get (Variables|Default|SetWBP_Tutorial%20Ref _returnvalue_3))
      (UserInterface|Viewport|AddtoViewport _output_get 0))
    (:then_2
      (Input|EnableInput (Game|GetPlayerController 0))
      (Input|EnableInput (Game|GetPlayerController 1)))))

(event EventTick
  (params (DeltaSeconds :type Float%20%28single-precision%29))
  (bind _wbp_tutorial_ref (Variables|Default|GetWBP_Tutorial%20Ref))
  (bind _wbp_tutorial_ref_2 (Variables|Default|GetWBP_Tutorial%20Ref))
  (bind _wbp_tutorial_ref_3 (Variables|Default|GetWBP_Tutorial%20Ref))
  (bind _wbp_tutorial_ref_4 (Variables|Default|GetWBP_Tutorial%20Ref))
  (bind _wbp_tutorial_ref_5 (Variables|Default|GetWBP_Tutorial%20Ref))
  (switch int (Variables|Default|GetTask_Counter)
    (:1
      (if (>= (Variables|Default|GetCompleted%20Task%20Number) 4)
        (Widget|SetVisibility (Variables|/Game/Dialogue/WBP_Tutorial.WBP_Tutorial_C|GetCanvas2 _wbp_tutorial_ref_4) "Hidden")
        (Widget|SetVisibility (Variables|/Game/Dialogue/WBP_Tutorial.WBP_Tutorial_C|Get6 _wbp_tutorial_ref_4) "Visible")
        (Widget|SetVisibility (Variables|/Game/Dialogue/WBP_Tutorial.WBP_Tutorial_C|Get6D _wbp_tutorial_ref_4) "Visible")
        (Variables|Default|SetTask_Counter 2)))
    (:3
      (if (> (Variables|Default|GetSpawned_Eco?) 0)
        (Variables|Default|SetENable%20Input%20Life false)
        (Widget|SetVisibility (Variables|/Game/Dialogue/WBP_Tutorial.WBP_Tutorial_C|Get7 _wbp_tutorial_ref_2) "Hidden")
        (Widget|SetVisibility (Variables|/Game/Dialogue/WBP_Tutorial.WBP_Tutorial_C|Get8 _wbp_tutorial_ref_2) "Visible")
        (Variables|Default|SetENable%20Input%20Death true)
        (Variables|Default|SetTask_Counter 4)))
    (:4
      (if (> (Variables|Default|GetSpawned_Graveyard?) 0)
        (Variables|Default|SetENable%20Input%20Death false)
        (Widget|SetVisibility (Variables|/Game/Dialogue/WBP_Tutorial.WBP_Tutorial_C|Get8 _wbp_tutorial_ref) "Hidden")
        (Widget|SetVisibility (Variables|/Game/Dialogue/WBP_Tutorial.WBP_Tutorial_C|Get9 _wbp_tutorial_ref) "Visible")
        (Widget|SetVisibility (Variables|/Game/Dialogue/WBP_Tutorial.WBP_Tutorial_C|Get9D _wbp_tutorial_ref) "Visible")
        (Variables|Default|SetTask_Counter 5)))
    (:12
      (bind _returnvalue (Actor|GetActorOfClass "/Game/Dialogue/BP_DeathTutorial.BP_DeathTutorial_C"))
      (if (Variables|/Game/Dialogue/BP_DeathTutorial.BP_DeathTutorial_C|GetAbility%201%20Done? _returnvalue)
        (Variables|/Game/Dialogue/BP_DeathTutorial.BP_DeathTutorial_C|SetCan%20Use%20ABility1? _returnvalue false)
        (Rendering|Material|CreateDynamicMaterialInstance (Variables|/Game/MapAssets/Blueprints/BP_HexGrid.BP_HexGrid_C|GetRed%20Tile (Variables|Default|GetAbility%201%20glow%20tile)) 0 "/Engine/EngineMaterials/WorldGridMaterial.WorldGridMaterial" "None" :!class /Script/Engine.PrimitiveComponent)
        (Widget|SetVisibility (Variables|/Game/Dialogue/WBP_Tutorial.WBP_Tutorial_C|Get18 _wbp_tutorial_ref_3) "Visible")
        (Widget|SetVisibility (Variables|/Game/Dialogue/WBP_Tutorial.WBP_Tutorial_C|Get19 _wbp_tutorial_ref_3) "Visible")
        (Variables|Default|SetTask_Counter 13)))
    (:13
      (bind _returnvalue_2 (Actor|GetActorOfClass "/Game/Dialogue/BP_DeathTutorial.BP_DeathTutorial_C"))
      (if (Variables|/Game/Dialogue/BP_DeathTutorial.BP_DeathTutorial_C|GetAbility%202%20Done? _returnvalue_2)
        (Variables|/Game/Dialogue/BP_DeathTutorial.BP_DeathTutorial_C|SetCan%20Use%20ABility2? _returnvalue_2 false)
        (Rendering|Material|CreateDynamicMaterialInstance (Variables|/Game/MapAssets/Blueprints/BP_HexGrid.BP_HexGrid_C|GetRed%20Tile (Variables|Default|GetAbility%202%20glow%20tile_0)) 0 "/Engine/EngineMaterials/WorldGridMaterial.WorldGridMaterial" "None" :!class /Script/Engine.PrimitiveComponent)
        (Widget|SetVisibility (Variables|/Game/Dialogue/WBP_Tutorial.WBP_Tutorial_C|Get20 _wbp_tutorial_ref_5) "Visible")
        (Widget|SetVisibility (Variables|/Game/Dialogue/WBP_Tutorial.WBP_Tutorial_C|Get20D _wbp_tutorial_ref_5) "Visible")
        (Variables|Default|SetTask_Counter 15)))))

(event Input|KeyboardEvents|L
  (params (Key :type Key%20Structure :default "None")))

(fn ConstructionScript)