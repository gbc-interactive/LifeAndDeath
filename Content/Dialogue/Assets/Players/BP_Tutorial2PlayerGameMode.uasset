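; Game mode for a two-player tutorial, with helper functions that check and remove entries in a TilesToGo collection.
; BeginPlay is empty, and the local multiplayer setup is disconnected, so it never runs.
; That unused chain would create a player per PlayerStart, giving player one the Life tutorial pawn and input mapping and others the Death equivalents.
; TakeT only tests membership despite its name, while RemoveOldTile does the removal.
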(event EventBeginPlay)

(fn ConstructionScript)

(fn TakeT
  (params (Tiletogo :type String))
  (return (Utilities|Array|ContainsItem (Variables|Default|GetTilesToGo) Tiletogo)))

(fn RemoveOldTile
  (params (CurrentTile :type String))
  (Utilities|Array|RemoveItem (Variables|Default|GetTilesToGo) CurrentTile)
  (return))

(fn NewFunction)