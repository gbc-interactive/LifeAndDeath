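; Game mode for the local two-player tutorial, setting up the Life and Death players when the level begins.
; BeginPlay creates a local player for each PlayerStart and possesses a pawn spawned there: BP_LifeTutorial for the first, BP_DeathTutorial for any others.
; Each player receives the matching IMC_Life or IMC_Death Enhanced Input mapping context.
; Helper functions check whether a tile is in TilesToGo and remove tiles from it.
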(event EventBeginPlay
  (bind _returnvalue (Game|GetPlayerController 0))
  (Development|PrintString "Level Begin")
  (bind _outactors (Actor|GetAllActorsOfClass "/Script/Engine.PlayerStart"))
  (for (_array_element _array_index) _outactors
    (bind _output_get (Variables|Default|SetArray%20Index _array_index))
    (bind _returnvalue_2 (Class|GameplayStatics|CreatePlayer _output_get))
    ;[1 1 1] Not Player 1
    (if (> (Variables|Default|GetArray%20Index) 0)
      (Input|AddMappingContext (PlayerController|LocalPlayerSubsystems|GetEnhancedInputLocalPlayerSubsystem _returnvalue_2) "/Game/TaskCharacter/ThirdPerson/Input/IMC_Death.IMC_Death" 0 "(bIgnoreAllPressedKeysUntilRelease=True,bForceImmediately=False,bNotifyUserSettings=False)")
      (bind _returnvalue_3 (Game|SpawnActorfromClass "/Game/Dialogue/BP_DeathTutorial.BP_DeathTutorial_C" (Transformation|GetActorTransform _array_element) "Undefined" "MultiplyWithRoot" 0 0))
      (Pawn|Possess (Game|GetPlayerController (Variables|Default|GetArray%20Index)) _returnvalue_3)
      (else
        ;[1 1 1] Player 1
        (Input|AddMappingContext (PlayerController|LocalPlayerSubsystems|GetEnhancedInputLocalPlayerSubsystem _returnvalue) "/Game/TaskCharacter/ThirdPerson/Input/IMC_Life.IMC_Life" 0 "(bIgnoreAllPressedKeysUntilRelease=True,bForceImmediately=False,bNotifyUserSettings=False)")
        (bind _returnvalue_4 (Game|SpawnActorfromClass "/Game/Dialogue/BP_LifeTutorial.BP_LifeTutorial_C" (Transformation|GetActorTransform _array_element) "Undefined" "MultiplyWithRoot" 0 0))
        (Pawn|Possess _returnvalue _returnvalue_4)))))

(fn ConstructionScript)

(fn TakeT
  (params (Tiletogo :type String))
  (return (Utilities|Array|ContainsItem (Variables|Default|GetTilesToGo) Tiletogo)))

(fn RemoveOldTile
  (params (CurrentTile :type String))
  (Utilities|Array|RemoveItem (Variables|Default|GetTilesToGo) CurrentTile)
  (return))

(fn NewFunction)