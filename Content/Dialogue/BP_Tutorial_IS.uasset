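; BP_Tutorial_IS is a tutorial character that tracks its movement and death state and highlights hex grid tiles under it.
; Tick derives moving and idle flags from velocity and sets IsDead when Health falls below 1.
; GlowBox overlaps swap each BP_HexGrid's RedTile material between Outline_Material and WorldGridMaterial.
; Talk is empty; the dialogue widget, camera blend and input-lock logic is disconnected and never runs.
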(event OnComponentBeginOverlap(Glowbox)
  (params (OverlappedComponent :type Primitive%20Component%20Object%20Reference) (OtherActor :type Actor%20Object%20Reference) (OtherComp :type Primitive%20Component%20Object%20Reference) (OtherBodyIndex :type Integer) (bFromSweep :type Boolean) (SweepResult :type Hit%20Result%20Structure%20%28by%20ref%29))
  ;[0.9655 1 0] Tile Glow
  (bind _asbp_hex_grid (Utilities|Casting|CastToBP_HexGrid OtherActor))
  (Rendering|Material|CreateDynamicMaterialInstance (Variables|/Game/MapAssets/Blueprints/BP_HexGrid.BP_HexGrid_C|GetRed%20Tile _asbp_hex_grid) 0 "/Game/MapAssets/Blueprints/Outline_Material.Outline_Material" "None" :!class /Script/Engine.PrimitiveComponent))

(event OnComponentEndOverlap(Glowbox)
  (params (OverlappedComponent :type Primitive%20Component%20Object%20Reference) (OtherActor :type Actor%20Object%20Reference) (OtherComp :type Primitive%20Component%20Object%20Reference) (OtherBodyIndex :type Integer))
  ;[0.9655 1 0] Tile Glow
  (bind _asbp_hex_grid (Utilities|Casting|CastToBP_HexGrid OtherActor))
  (Rendering|Material|CreateDynamicMaterialInstance (Variables|/Game/MapAssets/Blueprints/BP_HexGrid.BP_HexGrid_C|GetRed%20Tile _asbp_hex_grid) 0 "/Engine/EngineMaterials/WorldGridMaterial.WorldGridMaterial" "None" :!class /Script/Engine.PrimitiveComponent))

(event EventTalk
  ;[0.009027 1 0] Sets the Dialogue
)

(event EventTick
  (params (DeltaSeconds :type Float%20%28single-precision%29))
  (bind _returnvalue (Transformation|GetVelocity))
  (bind _returnvalue_2 (Math|Vector|VectorLength _returnvalue))
  (bind _returnvalue_3 (> _returnvalue_2 1.0))
  (Variables|Default|SetIsMoving _returnvalue_3)
  (Variables|Default|SetIsIdle (not _returnvalue_3))
  (if (< (Variables|Default|GetHealth) 1)
    (Variables|Default|SetIsDead true)))

(fn ConstructionScript)