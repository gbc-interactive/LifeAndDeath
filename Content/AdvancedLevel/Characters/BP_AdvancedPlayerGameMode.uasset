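; Game mode for the advanced level that sets up two local players, one as Life and one as Death.
; On BeginPlay it works around level restarts by destroying leftover Life and Death characters, including tutorial variants, and removing the second player.
; It then loops over PlayerStarts, creating players, adding each one's Enhanced Input mapping context, and spawning and possessing their character.
; Small helpers query and remove entries in a TilesToGo collection.
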(event EventBeginPlay
  (bind _returnvalue (Game|GetPlayerController 0))
  ;[1 1 1] This is a fix for level restart. Delete all actors and remove second pplayer so we can add it back in
  (bind _outactors (Actor|GetAllActorsOfClass "/Game/TaskCharacter/ThirdPerson/Blueprints/Life/BP_Life.BP_Life_C"))
  (Actor|DestroyActor _outactors)
  (bind _outactors_2 (Actor|GetAllActorsOfClass "/Game/Dialogue/BP_LifeTutorial.BP_LifeTutorial_C"))
  (Actor|DestroyActor _outactors_2)
  (bind _outactors_3 (Actor|GetAllActorsOfClass "/Game/AdvancedLevel/Characters/BP_AD_Life_Child.BP_AD_Life_Child_C"))
  (Actor|DestroyActor _outactors_3)
  (bind _outactors_4 (Actor|GetAllActorsOfClass "/Game/TaskCharacter/ThirdPerson/Blueprints/Death/BP_Death.BP_Death_C"))
  (Actor|DestroyActor _outactors_4)
  (bind _outactors_5 (Actor|GetAllActorsOfClass "/Game/AdvancedLevel/Characters/BP_ADDeath_Child.BP_ADDeath_Child_C"))
  (Actor|DestroyActor _outactors_5)
  (bind _outactors_6 (Actor|GetAllActorsOfClass "/Game/Dialogue/BP_DeathTutorial.BP_DeathTutorial_C"))
  (Actor|DestroyActor _outactors_6)
  (Class|GameplayStatics|RemovePlayer (Game|GetPlayerController 1) false)
  (bind _outactors_7 (Actor|GetAllActorsOfClass "/Script/Engine.PlayerStart"))
  (for (_array_element _array_index) _outactors_7
    (bind _output_get (Variables|Default|SetArray%20Index _array_index))
    (bind _returnvalue_2 (Class|GameplayStatics|CreatePlayer _output_get))
    ;[1 1 1] Not Player 1
    (if (> (Variables|Default|GetArray%20Index) 0)
      (Input|AddMappingContext (PlayerController|LocalPlayerSubsystems|GetEnhancedInputLocalPlayerSubsystem _returnvalue_2) "/Game/AdvancedLevel/Input/IMC_AdvancedDeath.IMC_AdvancedDeath" 0 "(bIgnoreAllPressedKeysUntilRelease=True,bForceImmediately=False,bNotifyUserSettings=False)")
      (bind _returnvalue_3 (Game|SpawnActorfromClass "/Game/AdvancedLevel/Characters/BP_ADDeath_Child.BP_ADDeath_Child_C" (Transformation|GetActorTransform _array_element) "Undefined" "MultiplyWithRoot" 0 0))
      (Pawn|Possess (Game|GetPlayerController (Variables|Default|GetArray%20Index)) _returnvalue_3)
      (else
        ;[1 1 1] Player 1
        (Input|AddMappingContext (PlayerController|LocalPlayerSubsystems|GetEnhancedInputLocalPlayerSubsystem _returnvalue) "/Game/AdvancedLevel/Input/IMC_AdvancedLife.IMC_AdvancedLife" 0 "(bIgnoreAllPressedKeysUntilRelease=True,bForceImmediately=False,bNotifyUserSettings=False)")
        (bind _returnvalue_4 (Game|SpawnActorfromClass "/Game/AdvancedLevel/Characters/BP_AD_Life_Child.BP_AD_Life_Child_C" (Transformation|GetActorTransform _array_element) "Undefined" "MultiplyWithRoot" 0 0))
        (Pawn|Possess _returnvalue _returnvalue_4)))))

(fn ConstructionScript)

(fn TakeT
  (params (Tiletogo :type String))
  (return (Utilities|Array|ContainsItem (Variables|Default|GetTilesToGo) Tiletogo)))

(fn RemoveOldTile
  (params (CurrentTile :type String))
  (Utilities|Array|RemoveItem (Variables|Default|GetTilesToGo) CurrentTile)
  (return))

(fn NewFunction)